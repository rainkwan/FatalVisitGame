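; BP_UsableDoor is a usable door that the player can open only when holding the matching key.
; OnUsed switches on DoorName across four doors, checking that door's HasKey flag on player 0's FirstPersonCharacter rather than the passed-in Character.
; With the key, it sets that door's Used flag, destroys the actor and clears KeyE.
; Without it, it sets NeedKey on the character.
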(event EventBeginPlay
  (|CallParentFunction) ; This node is disabled and will not be called.\nDrag off pins to build functionality.
)

(event Collision|EventActorBeginOverlap
  (params (OtherActor :type Actor%20Object%20Reference))
  (|CallParentFunction OtherActor) ; This node is disabled and will not be called.\nDrag off pins to build functionality.
)

(event EventTick
  (params (DeltaSeconds :type Float%20%28single-precision%29))
  (|CallParentFunction DeltaSeconds) ; This node is disabled and will not be called.\nDrag off pins to build functionality.
)

(fn ConstructionScript
  (|CallParentFunction))

(fn OnUsed
  (params (Character :type First%20Person%20Character%20Object%20Reference))
  (bind _asfirst_person_character (Utilities|Casting|CastToFirstPersonCharacter (Game|Player|GetPlayerPawn 0)))
  (switch string (Variables|Default|GetDoorName)
    (:Door1
      (if (Variables|/Game/FirstPersonBP/Blueprints/FirstPersonCharacter.FirstPersonCharacter_C|GetHasKey1 _asfirst_person_character)
        (Variables|/Game/FirstPersonBP/Blueprints/FirstPersonCharacter.FirstPersonCharacter_C|SetDoor1Used _asfirst_person_character true)
        (Actor|DestroyActor :!label _label)
        (Variables|/Game/FirstPersonBP/Blueprints/FirstPersonCharacter.FirstPersonCharacter_C|SetKeyE _asfirst_person_character false)
        (else
          (Variables|/Game/FirstPersonBP/Blueprints/FirstPersonCharacter.FirstPersonCharacter_C|SetNeedKey _asfirst_person_character true :!label _label_2))))
    (:Door2
      (if (Variables|/Game/FirstPersonBP/Blueprints/FirstPersonCharacter.FirstPersonCharacter_C|GetHasKey2 _asfirst_person_character)
        (Variables|/Game/FirstPersonBP/Blueprints/FirstPersonCharacter.FirstPersonCharacter_C|SetDoor2Used _asfirst_person_character true)
        (goto _label)
        (else
          (goto _label_2))))
    (:Door3
      (if (Variables|/Game/FirstPersonBP/Blueprints/FirstPersonCharacter.FirstPersonCharacter_C|GetHasKey3 _asfirst_person_character)
        (Variables|/Game/FirstPersonBP/Blueprints/FirstPersonCharacter.FirstPersonCharacter_C|SetDoor3Used _asfirst_person_character true)
        (goto _label)
        (else
          (goto _label_2))))
    (:Door4
      (if (Variables|/Game/FirstPersonBP/Blueprints/FirstPersonCharacter.FirstPersonCharacter_C|GetHasKey4 _asfirst_person_character)
        (Variables|/Game/FirstPersonBP/Blueprints/FirstPersonCharacter.FirstPersonCharacter_C|SetDoor4Used _asfirst_person_character true)
        (goto _label)
        (else
          (goto _label_2))))))