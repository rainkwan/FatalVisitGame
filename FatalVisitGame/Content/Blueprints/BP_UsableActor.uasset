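; BP_UsableActor is an interactable world object that highlights when the player focuses on it and disappears when used.
; BeginFocus and EndFocus toggle the "Lit" scalar material parameter on its static mesh and set the KeyE flag on the player's FirstPersonCharacter.
; OnUsed destroys the actor and clears KeyE.
; All three functions ignore their Character input and fetch player pawn 0 instead, and the event graph is empty.
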(event EventBeginPlay)

(event Collision|EventActorBeginOverlap
  (params (OtherActor :type Actor%20Object%20Reference)))

(event EventTick
  (params (DeltaSeconds :type Float%20%28single-precision%29)))

(fn ConstructionScript)

(fn EndFocus
  (params (Character :type First%20Person%20Character%20Object%20Reference))
  (Rendering|Material|SetScalarParameterValueonMaterials (Variables|Debug|GetStaticMeshComponent) "Lit" 0.0)
  (bind _asfirst_person_character (Utilities|Casting|CastToFirstPersonCharacter (Game|Player|GetPlayerPawn 0)))
  (Variables|/Game/FirstPersonBP/Blueprints/FirstPersonCharacter.FirstPersonCharacter_C|SetKeyE _asfirst_person_character false))

(fn BeginFocus
  (params (Character :type First%20Person%20Character%20Object%20Reference))
  (Rendering|Material|SetScalarParameterValueonMaterials (Variables|Debug|GetStaticMeshComponent) "Lit" 1.0)
  (bind _asfirst_person_character (Utilities|Casting|CastToFirstPersonCharacter (Game|Player|GetPlayerPawn 0)))
  (Variables|/Game/FirstPersonBP/Blueprints/FirstPersonCharacter.FirstPersonCharacter_C|SetKeyE _asfirst_person_character true))

(fn OnUsed
  (params (Character :type First%20Person%20Character%20Object%20Reference))
  (Actor|DestroyActor)
  (bind _asfirst_person_character (Utilities|Casting|CastToFirstPersonCharacter (Game|Player|GetPlayerPawn 0)))
  (Variables|/Game/FirstPersonBP/Blueprints/FirstPersonCharacter.FirstPersonCharacter_C|SetKeyE _asfirst_person_character false))