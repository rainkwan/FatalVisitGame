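; BP_GhostCharacter is the ghost enemy that triggers the player's death and game restart when the player is within range.
; It caches the FirstPersonCharacter on BeginPlay and asks it every Tick whether the ghost is within range.
; A catch or a won game teleports the ghost to OriginalGhostLocation, which this file never sets.
; PlayerInFinalRoom is a distance check to the player that nothing here calls.
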(event EventBeginPlay
  (bind _asfirst_person_character (Utilities|Casting|CastToFirstPersonCharacter (Game|Player|GetPlayerPawn 0)))
  (Variables|Default|SetCharacter _asfirst_person_character))

(event Collision|EventActorBeginOverlap
  (params (OtherActor :type Actor%20Object%20Reference)))

(event EventTick
  (params (DeltaSeconds :type Float%20%28single-precision%29))
  (bind _character (Variables|Default|GetCharacter))
  (bind _withinrange (Default|WithinRange _character self))
  (if _withinrange
    (Default|RestartGameonDeath _character)
    (Transformation|SetActorLocation (Variables|Default|GetOriginalGhostLocation) false true :!label _label)
    (elif (Variables|/Game/FirstPersonBP/Blueprints/FirstPersonCharacter.FirstPersonCharacter_C|GetWonGameBool (Variables|Default|GetCharacter))
      (goto _label))))

(fn ConstructionScript)

(fn PlayerinFinalRoom
  (return (< (Math|Vector|Distance(Vector) (Transformation|GetActorLocation (Variables|Default|GetCharacter)) (Transformation|GetActorLocation)) 1e+03)))